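; Player character Blueprint that handles ground movement, camera look, sprinting and firing through Enhanced Input.
; BeginPlay adds the ground character mapping context to the possessing player controller.
; Movement follows control yaw, while holding sprint raises walk speed and restricts input to forward only, blocking strafing and backpedaling.
; Fire input only plays a montage on the mesh.
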(event Input|EnhancedActionEvents|EnhancedInputActionIA_my_groundmove
  (params (ActionValue :type Vector%202D%20Structure) (ElapsedSeconds :type Float%20%28double-precision%29) (TriggeredSeconds :type Float%20%28double-precision%29) (InputAction :type Input%20Action%20Object%20Reference :default "/Game/input/IA_my_groundmove.IA_my_groundmove"))
  (bind _returnvalue (Pawn|GetControlRotation :!class /Script/Engine.Pawn))
  (bind _returnvalue_2 (Pawn|GetControlRotation :!class /Script/Engine.Pawn))
  (bind _returnvalue_3 (Math|Vector|GetForwardVector (Math|Rotator|MakeRotator 0.0 0.0 (.yaw _returnvalue))))
  (:Triggered
    (Pawn|Input|AddMovementInput (Math|Vector|GetRightVector (Math|Rotator|MakeRotator (.roll _returnvalue_2) 0.0 (.yaw _returnvalue_2))) (* (Math|Conversions|ToFloat(Boolean) (not (Variables|Default|Getissprint))) (.x ActionValue)) false)
    (if (Variables|Default|Getissprint)
      (Pawn|Input|AddMovementInput _returnvalue_3 (Math|Float|SelectFloat (.y ActionValue) 0.0 (> (.y ActionValue) 0.0)) false)
      (else
        (Pawn|Input|AddMovementInput _returnvalue_3 (.y ActionValue) false)))))

(event Input|EnhancedActionEvents|EnhancedInputActionIA_my_camrotate
  (params (ActionValue :type Vector%202D%20Structure) (ElapsedSeconds :type Float%20%28double-precision%29) (TriggeredSeconds :type Float%20%28double-precision%29) (InputAction :type Input%20Action%20Object%20Reference :default "/Game/input/IA_my_camrotate.IA_my_camrotate"))
  (:Triggered
    (Pawn|Input|AddControllerYawInput (.x ActionValue))
    (Pawn|Input|AddControllerPitchInput (.y ActionValue))))

(event Input|EnhancedActionEvents|EnhancedInputActionia_my_Sprint
  (params (ActionValue :type Boolean) (ElapsedSeconds :type Float%20%28double-precision%29) (TriggeredSeconds :type Float%20%28double-precision%29) (InputAction :type Input%20Action%20Object%20Reference :default "/Game/input/ia_my_Sprint.ia_my_Sprint"))
  (bind _charactermovement (Variables|Character|GetCharacterMovement))
  (:Started
    (Variables|/Script/Engine.CharacterMovementComponent|SetMaxWalkSpeed _charactermovement 6e+02)
    (Variables|Default|Setissprint true))
  (:Completed
    (Variables|/Script/Engine.CharacterMovementComponent|SetMaxWalkSpeed _charactermovement 3e+02)
    (Variables|Default|Setissprint false)))

(event Input|EnhancedActionEvents|EnhancedInputActionIA_my_fire
  (params (ActionValue :type Boolean) (ElapsedSeconds :type Float%20%28double-precision%29) (TriggeredSeconds :type Float%20%28double-precision%29) (InputAction :type Input%20Action%20Object%20Reference :default "/Game/input/IA_my_fire.IA_my_fire"))
  (:Triggered
    (Animation|Montage|PlayMontage (Variables|Character|GetMesh) "/Game/MT_MY_FIRE.MT_MY_FIRE")))

(event EventBeginPlay
  (bind _as플레이어_컨트롤러 (Utilities|Casting|CastToPlayerController (Pawn|GetController)))
  (Utilities|IsValid (PlayerController|LocalPlayerSubsystems|GetEnhancedInputLocalPlayerSubsystem _as플레이어_컨트롤러)
    (:Is%20Valid
      (Input|AddMappingContext (PlayerController|LocalPlayerSubsystems|GetEnhancedInputLocalPlayerSubsystem _as플레이어_컨트롤러) "/Game/input/imc_MY_groundchara.imc_MY_groundchara" 0 "(bIgnoreAllPressedKeysUntilRelease=True,bForceImmediately=False)"))))

(event Collision|EventActorBeginOverlap
  (params (OtherActor :type Actor%20Object%20Reference)))

(event EventTick
  (params (DeltaSeconds :type Float%20%28single-precision%29)))

(fn ConstructionScript)